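; Actor component that makes its owner float up and down along world Z.
; BeginPlay caches the owner and its start location, then Tick offsets that location by a sine of game time scaled by Frequency and Amplitude.
; Each tick sets the absolute position without sweep, pinning X and Y to the cached start.
; TurnOn enables ticking and recaptures the current location as the new origin, while TurnOff disables ticking.
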(event `self.ReceiveBeginPlay`
  (bind _output_get (set `self.ParentActor` (`self.GetOwner`)))
  (set `self.Start Location` (`Actor.K2_GetActorLocation` _output_get)))

(event `self.ReceiveTick`
  (params (DeltaSeconds :type "Float (single-precision)"))
  (`Actor.K2_SetActorLocation` (`self.ParentActor`) (+ (`self.Start Location`) (`KismetMathLibrary.MakeVector` 0.0 0.0 (* (`KismetMathLibrary.Sin` (* (`self.Frequency`) (`GameplayStatics.GetTimeSeconds`) 6.283184)) (`self.Amplitude`)))) false false))

(fn `Turn Off`
  (`self.SetComponentTickEnabled` false))

(fn `TurnOn`
  (`self.SetComponentTickEnabled` true)
  (set `self.Start Location` (`Actor.K2_GetActorLocation` (`self.ParentActor`))))